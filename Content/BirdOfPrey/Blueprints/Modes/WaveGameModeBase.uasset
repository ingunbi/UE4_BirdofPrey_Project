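; Base game mode for wave-based scrolling shooter modes, configurable for time-limited, boss rush or open-ended play.
; A one-second looping timer drives status text, scroll stop, win checks and spawning of growing waves from a widening enemy pool.
; Bosses arrive at wave intervals or sequentially in boss rush, and enemies spawn just beyond the camera's view.
; Enemy deaths award score, attempt power-up drops and advance boss progress.
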(event EventBeginPlay
  (|CallParentFunction) ; 지금 이 노드는 비활성 상태입니다. \n핀을 끌어서 다른 노드를 연결하면 활성화됩니다.
)

(event EventTick
  (params (DeltaSeconds :type Float%20%28single-precision%29)))

(fn ConstructionScript
  (|CallParentFunction))

(fn SpawnEnemyat
  (params (EnemyClass :type Base%20Game%20Agent%20Class%20Reference) (YFraction :type Float%20%28double-precision%29))
  (bind _worldcameraactor (CallFunction|GetWorldCameraActor))
  (bind _returnvalue (Transformation|GetActorLocation _worldcameraactor))
  (bind (_height _width) (Default|GetScreenDimensions _worldcameraactor))
  (bind (_x _y) (Math|Vector|BreakVector _returnvalue))
  (bind _returnvalue_2 (Game|SpawnActorfromClass :Class EnemyClass :SpawnTransform (Math|Transform|MakeTransform (Math|Vector|MakeVector (+ (+ _x (* _height 0.5)) 1.5e+02) (+ _y (* YFraction _width)) (Variables|Default|GetSpawnHeight)) (Math|Rotator|MakeRotator 0.0 0.0 1.8e+02)) :CollisionHandlingOverride "AlwaysSpawn" :TransformScaleMethod "MultiplyWithRoot" :Instigator 0))
  (return _returnvalue_2))

(fn SpawnBoss
  (params (BossClass :type Base%20Game%20Agent%20Class%20Reference))
  (CallFunction|SpawnEnemyat BossClass 0.0)
  (Variables|Default|SetbBossAlive true)
  (return))

(fn SpawnWave
  (bind _enemypool (Variables|Default|GetEnemyPool))
  (bind _bossevery (Variables|Default|GetBossEvery))
  (bind _bosspool (Variables|Default|GetBossPool))
  (bind _returnvalue (Math|Integer|Max(Integer) _bossevery 1))
  (bind _output_get (Variables|Default|SetWave (+ (Variables|Default|GetWave) 1)))
  (for _index (range 1 (Math|Integer|Min(Integer) (+ 2 _output_get) (Variables|Default|GetMaxPerWave)))
    (CallFunction|SpawnEnemyat (Utilities|Array|Get(acopy) _enemypool (Math|Random|RandomIntegerinRange 0 (Math|Integer|Min(Integer) (+ (/ _output_get 2) 1) (- (Utilities|Array|Length _enemypool) 1)))) (Math|Random|RandomFloatinRange -0.4 0.4)))
  (if (and (and (> _bossevery 0) (== (Math|Integer|%(Integer) _output_get _returnvalue) 0)) (not (Variables|Default|GetbBossAlive)))
    (CallFunction|SpawnBoss (Utilities|Array|Get(acopy) _bosspool (Math|Integer|%(Integer) (/ _output_get _returnvalue) (Utilities|Array|Length _bosspool)))))
  (return))

(fn FormatTime
  (params (Seconds :type Float%20%28double-precision%29))
  (return (Utilities|String|GetSubstring (Class|KismetStringLibrary|TimeSecondstoString Seconds) 0 5)))

(fn UpdateStatus
  (bind _timelimit (Variables|Default|GetTimeLimit))
  (bind _elapsedtime (Variables|Default|GetElapsedTime))
  (bind _wave (Variables|Default|GetWave))
  (bind _bosspool (Variables|Default|GetBossPool))
  (bind _returnvalue (Utilities|Array|Length _bosspool))
  (if (> _timelimit 0.0)
    (Variables|Default|SetStatusText (Utilities|String|Append (Utilities|String|Append (Utilities|String|Append "TIME LEFT " (CallFunction|FormatTime (- _timelimit _elapsedtime))) "   WAVE ") (Utilities|String|ToString(Integer) _wave)))
    (elif (Variables|Default|GetbBossRush)
      (Variables|Default|SetStatusText (Utilities|String|Append (Utilities|String|Append (Utilities|String|Append "BOSS " (Utilities|String|ToString(Integer) (Math|Integer|Min(Integer) (+ (Variables|Default|GetBossesDefeated) 1) _returnvalue))) " / ") (Utilities|String|ToString(Integer) _returnvalue)))
      (else
        (Variables|Default|SetStatusText (Utilities|String|Append (Utilities|String|Append (Utilities|String|Append "WAVE " (Utilities|String|ToString(Integer) _wave)) "   TIME ") (CallFunction|FormatTime _elapsedtime))))))
  (return))

(fn ModeTick
  (bind _timelimit (Variables|Default|GetTimeLimit))
  (bind _bossesdefeated (Variables|Default|GetBossesDefeated))
  (bind _bosspool (Variables|Default|GetBossPool))
  (if (Variables|Default|GetIsGameOverScreen)
    (return)
    (else
      (bind _output_get (Variables|Default|SetElapsedTime (+ (Variables|Default|GetElapsedTime) 1.0)))
      (if (and (> _timelimit 0.0) (>= _output_get _timelimit))
        (CallFunction|UpdateStatus)
        (CallFunction|EndGame true)
        (else
          (if (> (CallFunction|GetDistanceTravelled) (Variables|Default|GetMaxScrollDistance))
            (Variables|Default|SetWorldScrollSpeed 0.0))
          (if (and (and (and (Variables|Default|GetbBossRush) (not (Variables|Default|GetbBossAlive))) (< _bossesdefeated (Utilities|Array|Length _bosspool))) (>= _output_get (Variables|Default|GetNextBossTime)))
            (CallFunction|SpawnBoss (Utilities|Array|Get(acopy) _bosspool _bossesdefeated)))
          (if (== (Math|Integer|%(Integer) (Math|Float|Truncate _output_get) (Variables|Default|GetWaveInterval)) 0)
            (CallFunction|SpawnWave))
          (CallFunction|UpdateStatus))))))

(fn OnEnemyDied
  (params (Enemy :type Base%20Game%20Agent%20Object%20Reference) (Killer :type Controller%20Object%20Reference))
  (if (Utilities|IsValid Enemy)
    (if (Utilities|IsValid Killer)
      (bind _asbase_player_state (Utilities|Casting|CastToBasePlayerState (Variables|/Script/Engine.Controller|GetPlayerState Killer))
        (:then
          (Default|AddScore _asbase_player_state (Variables|/Game/BirdOfPrey/Blueprints/BaseGameAgent.BaseGameAgent_C|GetPoints Enemy))
          (CallFunction|TrySpawnPowerUp (Transformation|GetActorLocation Enemy)))
        (:CastFailed
          _)))
    (Utilities|Casting|CastToBaseBossShip Enemy
      (:then
        (Variables|Default|SetbBossAlive false)
        (bind _output_get (Variables|Default|SetBossesDefeated (+ (Variables|Default|GetBossesDefeated) 1)))
        (Variables|Default|SetNextBossTime (+ (Variables|Default|GetElapsedTime) (Variables|Default|GetBossDelay)))
        (if (and (Variables|Default|GetbBossRush) (>= _output_get (Utilities|Array|Length (Variables|Default|GetBossPool))))
          (CallFunction|UpdateStatus)
          (CallFunction|EndGame true)
          (else
            (CallFunction|UpdateStatus)
            (return))))
      (:CastFailed
        (return)))
    (else
      (return))))

(fn StartGame
  (|CallParentFunction)
  (Variables|Default|SetWave 0)
  (Variables|Default|SetElapsedTime 0.0)
  (Variables|Default|SetBossesDefeated 0)
  (Variables|Default|SetbBossAlive false)
  (Variables|Default|SetNextBossTime 3.0)
  (Variables|Default|SetWorldScrollSpeed (Variables|Default|GetModeScrollSpeed))
  (Utilities|Time|SetTimerbyFunctionName self "ModeTick" 1.0 true)
  (CallFunction|UpdateStatus))