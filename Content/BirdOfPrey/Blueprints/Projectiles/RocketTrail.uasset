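; RocketTrail is a spline-based projectile actor that builds a trail out of spline mesh pieces.
; The construction script divides the Spline's length by PieceLength and adds a SplineMeshComponent for each step.
; Each piece takes local-space positions and raw, unscaled tangents from the spline at its two end distances.
; The event graph has no active logic, so the trail is built only at construction.
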(event EventBeginPlay)

(event Collision|EventActorBeginOverlap
  (params (OtherActor :type Actor%20Object%20Reference)))

(event EventTick
  (params (DeltaSeconds :type Float%20%28single-precision%29)))

(fn ConstructionScript
  (bind _piecelength (Variables|Default|GetPieceLength))
  (bind _spline (Variables|Default|GetSpline))
  (for _index (range 0 (Math|Float|Truncate (/ (Spline|GetSplineLength (Variables|Default|GetSpline)) (Variables|Default|GetPieceLength))))
    (bind _returnvalue (AddComponent|AddSplineMeshComponent false))
    (SplineMesh|SetStartandEnd _returnvalue (Spline|GetLocationatDistanceAlongSpline _spline (* _index _piecelength) "Local") (Spline|GetTangentatDistanceAlongSpline _spline (* _index _piecelength) "Local") (Spline|GetLocationatDistanceAlongSpline _spline (+ (* _index _piecelength) _piecelength) "Local") (Spline|GetTangentatDistanceAlongSpline _spline (+ (* _index _piecelength) _piecelength) "Local") true :!class /Script/Engine.SplineMeshComponent)))