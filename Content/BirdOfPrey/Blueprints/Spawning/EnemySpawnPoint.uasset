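; Placed spawn point that spawns one enemy of its configured type when the world camera approaches it along X.
; A looping timer with a randomized interval compares its X distance to the camera against half the screen height plus an offset, using the camera from BaseGameMode.
; Spawning uses the point's location and rotation, ignores collisions and clears the timer.
; Reset restarts the check so the point can spawn again.
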(event EventBeginPlay
  ;[1 1 1] Begin Play
  (bind _asbase_game_mode (Utilities|Casting|CastToBaseGameMode (Game|GetGameMode)))
  (Variables|Default|SetGameMode _asbase_game_mode)
  (CallFunction|StartCheckingforSpawns))

(event EventReset
  ;[1 1 1] Handle Reset
  (CallFunction|StartCheckingforSpawns))

(fn ConstructionScript)

(fn SpawnEnemy
  (Game|SpawnActorfromClass :Class (Variables|Default|GetEnemyType) :SpawnTransform (Math|Transform|MakeTransform (Transformation|GetActorLocation) (Transformation|GetActorRotation) "1.000000,1.000000,1.000000") :CollisionHandlingOverride "AlwaysSpawn" :TransformScaleMethod "SelectDefaultAtRuntime" :Instigator 0)
  (Utilities|Time|ClearandInvalidateTimerbyHandle (Variables|Default|GetSpawnTimerHandle)))

(fn CheckforSpawn
  (bind _gamemode (Variables|Default|GetGameMode))
  (bind _worldcameraactor (Default|GetWorldCameraActor _gamemode))
  (if (< (- (.x (Transformation|GetActorLocation)) (.x (Transformation|GetActorLocation _worldcameraactor))) (+ (/ (.Height (Default|GetScreenDimensions _worldcameraactor)) 2.0) (Variables|Default|GetSpawnDistanceOffset)))
    (CallFunction|SpawnEnemy)))

(fn StartCheckingforSpawns
  (bind _returnvalue (Utilities|Time|SetTimerbyEvent (EventDispatchers|CreateEvent :!event CheckforSpawn) (+ 0.2 (Math|Random|RandomFloatinRange -0.1 0.1)) true))
  (Variables|Default|SetSpawnTimerHandle _returnvalue))