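; BaseShip is a base Blueprint for ships, extending a parent agent class with ship-specific attachment and speed.
; On BeginPlay it attaches itself to the game mode's world camera actor, keeping world transforms, so it moves with the scrolling world.
; It overrides ApplyAgentInfo to run the parent logic, then copy the agent's Speed into the FloatingPawnMovement max speed.
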(event EventBeginPlay
  (|CallParentFunction)
  (Transformation|AttachActorToActor (Default|GetWorldCameraActor (.AsBase%20Game%20Mode (Utilities|Casting|CastToBaseGameMode (Game|GetGameMode)))) "None" "KeepWorld" "KeepWorld" "KeepWorld" true) ; When we spawn a ship we want to add it to the camera actor so it moves with the world
)

(event Collision|EventActorBeginOverlap
  (params (OtherActor :type Actor%20Object%20Reference)))

(event EventTick
  (params (DeltaSeconds :type Float%20%28single-precision%29)))

(event EventApplyAgentInfo
  (params (NewAgentInfo :type Agent%20Info%20Structure))
  (|CallParentFunction NewAgentInfo)
  (Variables|/Script/Engine.FloatingPawnMovement|SetMaxSpeed (Variables|Default|GetFloatingPawnMovement) (.Speed (Utilities|Struct|BreakAgentInfo NewAgentInfo))))

(fn ConstructionScript
  (|CallParentFunction))