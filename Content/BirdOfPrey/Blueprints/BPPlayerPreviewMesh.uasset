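; Player preview mesh that shows the selected agent's skeletal mesh, scale, colour and animation class.
; On BeginPlay it binds to the game instance's agent-info change event and shows player 0's agent, falling back to the "Light" data table row.
; Each update first clears material overrides so they don't carry onto the incoming mesh, and applies changes regardless of which player controller ID is passed.
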(event Custom|UpdateMesh
  (params (PlayerControllerID :type Integer) (AgentInfo :type Agent%20Info%20Structure))
  (bind (_skeletalmesh _animinstance _meshscale _colour) (Utilities|Struct|BreakAgentInfo AgentInfo))
  (bind _skeletalmeshcomponent (Variables|SkeletalMeshActor|GetSkeletalMeshComponent))
  (bind _skeletalmeshcomponent_2 (Variables|SkeletalMeshActor|GetSkeletalMeshComponent))
  (Utilities|FlowControl|Sequence
    (:then_0
      ;[1 1 1] Clear Existing Materials so that they don't override the incoming mesh
      (for (_ _array_index) (Rendering|Material|GetMaterials _skeletalmeshcomponent)
        (Rendering|Material|SetMaterial _skeletalmeshcomponent _array_index 0)))
    (:then_1
      (Components|SkinnedMesh|SetSkinnedAssetandUpdate _skeletalmeshcomponent_2 _skeletalmesh true)
      (Transformation|SetWorldScale3D _skeletalmeshcomponent_2 (Math|Conversions|ToVector(Float) _meshscale))
      (Rendering|Material|SetVectorParameterValueonMaterials (Variables|SkeletalMeshActor|GetSkeletalMeshComponent) "BaseColour" (Math|Conversions|ToVector(LinearColor) _colour))
      (Components|SkeletalMesh|SetAnimInstanceClass (Variables|SkeletalMeshActor|GetSkeletalMeshComponent) _animinstance))))

(event EventBeginPlay
  (bind _asbase_game_instance (Utilities|Casting|CastToBaseGameInstance (Game|GetGameInstance)))
  (EventDispatchers|BindEventtoOnAgentInfoChange _asbase_game_instance (delegate Custom|UpdateMesh))
  (bind (_returnvalue _success) (Default|GetPlayerAgentInfofor _asbase_game_instance))
  (if _success
    (CallFunction|UpdateMesh 0 _returnvalue)
    (else
      (bind _returnvalue_2 (Utilities|GetDataTableRow "/Game/BirdOfPrey/Blueprints/AgentData/PlayerAgentInfoDataTable.PlayerAgentInfoDataTable" "Light")
        (:then
          (CallFunction|UpdateMesh 0 _returnvalue_2))))))

(fn ConstructionScript)