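; Utility function library for BirdOfPrey with a single check, IsOnScreen, that tests whether an agent lies within the visible play area.
; It builds a box around the world camera actor from the game mode, using half the screen height on X and half the width on Y, padded by a tolerance and given a fixed Z extent.
; If the game mode is not a BaseGameMode, it reports the agent as on screen.
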(fn IsonScreen
  (params (Agent :type Base%20Game%20Agent%20Object%20Reference) (Tolerance :type Float%20%28double-precision%29))
  (bind _asbase_game_mode (Utilities|Casting|CastToBaseGameMode (Game|GetGameMode Agent))
    (:then
      (return (Math|Geometry|IsPointinBox (Transformation|GetActorLocation Agent) (Transformation|GetActorLocation (Default|GetWorldCameraActor _asbase_game_mode)) (Math|Vector|MakeVector (+ (/ (.Height (Default|GetScreenDimensions (Default|GetWorldCameraActor _asbase_game_mode))) 2.0) Tolerance) (+ (/ (.Width (Default|GetScreenDimensions (Default|GetWorldCameraActor _asbase_game_mode))) 2.0) Tolerance) 1e+03))))
    (:CastFailed
      (return true))))