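; HealthPowerUp is a power-up Blueprint that restores health to the player ship.
; It overrides Apply, calling the parent version and then adding a fixed amount to the ship's Health, capped at the Health value in its AgentInfo.
; Its event graph holds only disabled placeholder events, and construction defers to the parent.
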(event EventBeginPlay)

(event Collision|EventActorBeginOverlap
  (params (OtherActor :type Actor%20Object%20Reference))
  (|CallParentFunction OtherActor) ; 지금 이 노드는 비활성 상태입니다. \n핀을 끌어서 다른 노드를 연결하면 활성화됩니다.
)

(event EventTick
  (params (DeltaSeconds :type Float%20%28single-precision%29)))

(fn ConstructionScript
  (|CallParentFunction))

(fn Apply
  (params (PlayerShip :type Player%20Ship%20Object%20Reference))
  (|CallParentFunction PlayerShip)
  (Variables|/Game/BirdOfPrey/Blueprints/BaseGameAgent.BaseGameAgent_C|SetHealth PlayerShip (Math|Float|Min(Float) (+ (Variables|/Game/BirdOfPrey/Blueprints/BaseGameAgent.BaseGameAgent_C|GetHealth PlayerShip) 1e+02) (.Health (Utilities|Struct|BreakAgentInfo (Variables|/Game/BirdOfPrey/Blueprints/BaseGameAgent.BaseGameAgent_C|GetAgentInfo PlayerShip))))))